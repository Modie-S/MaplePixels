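; BP_CharacterBase is a base character Blueprint that shows floating damage numbers over damaged actors.
; DisplayFloatingText forwards to an SRV-prefixed event, which spawns BP_FloatingText slightly above the damaged actor.
; A switch on text type reads player or enemy damage from that actor via reference messages, then sets the number, icon and colour.
; GetCharacterRef returns the character itself.
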(event Custom|SRV_DisplayFloatingText
  (params (DamagedActor :type Actor%20Object%20Reference) (FloatingTextType :type E_FloatingTextType%20Enum :default "NewEnumerator0"))
  (bind _output_get (Variables|Default|SetDamaged%20Actor DamagedActor))
  (bind _returnvalue (Game|SpawnActorfromClass "/Game/Blueprints/BP_FloatingText.BP_FloatingText_C" (Math|Transform|MakeTransform (Math|Vector|MakeVector (.X (Math|Vector|BreakVector (Transformation|GetActorLocation _output_get))) (.Y (Math|Vector|BreakVector (Transformation|GetActorLocation _output_get))) (+ (.Z (Math|Vector|BreakVector (Transformation|GetActorLocation _output_get))) 3e+01))) "AdjustIfPossibleButAlwaysSpawn" 0 0))
  (bind _output_get_2 (Variables|Default|SetFloatingText _returnvalue))
  (switch Utilities|FlowControl|Switch|SwitchonE_FloatingTextType FloatingTextType
    (:NewEnumerator0
      (bind _enemy (Class|INTEnemyBase|GetEnemyRef(Message) (Variables|Default|GetDamaged%20Actor)))
      (Default|DisplayFloatingText _output_get_2 (Utilities|Text|ToText(Float) (Variables|/Game/Blueprints/Enemy/BP_EnemyBase.BP_EnemyBase_C|GetPlayerDamageAmount _enemy) "HalfToEven") "/Game/UI/Images/IMG_Sword.IMG_Sword" "(R=0.286458,G=0.715539,B=1.000000,A=1.000000)"))
    (:NewEnumerator1
      (bind _player (Class|INTPlayerBase|GetPlayerRef(Message) (Variables|Default|GetDamaged%20Actor)))
      (Default|DisplayFloatingText _output_get_2 (Utilities|Text|ToText(Float) (Variables|/Game/Blueprints/Player/BP_PlayerBase.BP_PlayerBase_C|GetEnemyDamageAmount _player) "HalfToEven") "/Game/UI/Images/IMG_Blood.IMG_Blood" "(R=1.000000,G=0.208333,B=0.337637,A=1.000000)"))))

(event EventDisplayFloatingText
  (params (DamagedActor :type Actor%20Object%20Reference) (FloatingTextType :type E_FloatingTextType%20Enum :default "NewEnumerator0"))
  (CallFunction|SRVDisplayFloatingText DamagedActor FloatingTextType))

(fn ConstructionScript)

(fn GetCharacterRef
  (return self))